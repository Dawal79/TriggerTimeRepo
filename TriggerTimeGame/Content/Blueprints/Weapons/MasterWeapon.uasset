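; Base weapon actor that players can pick up through the interactor's weapon system component and fire.
; An overlap area shows an interact widget with the weapon's name, while SetWeaponState switches collision and physics for dropped, equipped and holding states.
; StartFire passes a gate once per call and, with ammo left, line-traces from the follow camera.
; GunEffects plays sound and a montage; no damage or ammo deduction happens here.
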(event `self.InteractArea.OnComponentBeginOverlap`
  (params (OverlappedComponent :type "PrimitiveComponent Object Reference") (OtherActor :type "Actor Object Reference") (OtherComp :type "PrimitiveComponent Object Reference") (OtherBodyIndex :type Integer) (bFromSweep :type Boolean) (SweepResult :type "HitResult Structure (by ref)"))
  (bind _widget (`self.Widget`))
  (cast `/Game/ThirdPerson/Blueprints/BP_ThirdPersonCharacter` OtherActor)
  (set `self.canPick` true)
  (`self.interactUI`
    (:`then`
      _)
    (:`else`
      (bind _returnvalue (`|CreateWidget` "/Game/Blueprints/UI/WBP_Interact.WBP_Interact_C" null (`.WeaponName_2_2B29DAA54443E25F4038048285F510E0` (break `/Game/Blueprints/Weapons/WeaponStruc` (`self.weaponStruct`)))))
      (bind _output_get (set `self.interactUI` _returnvalue))
      (`WidgetComponent.SetWidget` _widget _output_get)))
  (`SceneComponent.SetVisibility` _widget true false))

(event `self.InteractArea.OnComponentEndOverlap`
  (params (OverlappedComponent :type "PrimitiveComponent Object Reference") (OtherActor :type "Actor Object Reference") (OtherComp :type "PrimitiveComponent Object Reference") (OtherBodyIndex :type Integer))
  (`SceneComponent.SetVisibility` (`self.Widget`) false false)
  (set `self.canPick` false))

(event `/Game/Blueprints/InteractInterface.Interact`
  (params (Interactor :type "Actor Object Reference"))
  (set `self.Interactor` Interactor)
  (`/Game/Blueprints/Weapons/WeaponSysremComponent.PickupWeapon` (`self.GetComponentByClass` Interactor "/Game/Blueprints/Weapons/WeaponSysremComponent.WeaponSysremComponent_C") self)
  (bind _asbp_third_person_character (cast `/Game/ThirdPerson/Blueprints/BP_ThirdPersonCharacter` (`self.Interactor`)))
  (set `self.PlayerRef` _asbp_third_person_character))

(event `StartFire`
  (bind (_start _end) (`self.StartAndEndPoint`))
  (`|ExecutionSequence`
    (:`then_0`
      (goto _label :!via `Open`))
    (:`then_1`
      (`/Engine/EditorBlueprintResources/StandardMacros.Gate` true :!label _label
        (:`Exit`
          (if (> (`.CurrentAmmo_14_FCF11E774CA6763FCD47E1BFFACF68EC` (break `/Game/Blueprints/Weapons/WeaponStruc` (`self.weaponStruct`))) 0)
            (bind (_outhit _returnvalue) (`KismetSystemLibrary.LineTraceSingle` _start _end "TraceTypeQuery3" false (`|MakeArray` (`self.Interactor`)) "ForDuration"))
            (bind (_bblockinghit _binitialoverlap _time _distance _location _impactpoint _normal _impactnormal _physmat _hitactor _hitcomponent _hitbonename _bonename _hititem _elementindex _faceindex _tracestart _traceend) (`GameplayStatics.BreakHitResult` _outhit))
            (`self.GunEffects` _returnvalue _impactnormal (select `bool` _returnvalue :`false` _traceend :`true` _impactpoint))))))))

(event `StopFire`
  (goto _label :!via `Close`))

(fn `GunEffects`
  (params (HasHit :type Boolean) (ImpactPoint :type "Vector Structure") (TraceEnd :type "Vector Structure") (NewParam :type "Vector Structure"))
  (`GameplayStatics.PlaySound2D` (`self.ShootSound`) 1.0 1.0 0.0 null null)
  (`Character.PlayAnimMontage` (`self.PlayerRef`) (`self.Anim Montage`) 0.6 "None"))

(fn `SetWeaponState`
  (params (WeaponState :type "/Game/Blueprints/Weapons/E_WeaponState Enum" :default "NewEnumerator0"))
  (bind _weaponmesh (`self.WeaponMesh`))
  (switch `/Game/Blueprints/Weapons/E_WeaponState` WeaponState
    (:`NewEnumerator0`
      (`PrimitiveComponent.SetCollisionProfileName` (`self.InteractArea`) "OverlapAllDynamic" true)
      (`PrimitiveComponent.SetCollisionProfileName` (`self.WeaponMesh`) "DroppedGun" true)
      (`PrimitiveComponent.SetSimulatePhysics` (`self.WeaponMesh`) true))
    (:`NewEnumerator1`
      (`PrimitiveComponent.SetCollisionProfileName` (`self.InteractArea`) "NoCollision" true)
      (`PrimitiveComponent.SetCollisionProfileName` (`self.WeaponMesh`) "NoCollision" true)
      (`PrimitiveComponent.SetSimulatePhysics` _weaponmesh false)
      (`SceneComponent.ResetRelativeTransform` _weaponmesh))
    (:`NewEnumerator2`
      (`PrimitiveComponent.SetCollisionProfileName` (`self.InteractArea`) "NoCollision" true)
      (`PrimitiveComponent.SetCollisionProfileName` (`self.WeaponMesh`) "NoCollision" true)
      (`PrimitiveComponent.SetSimulatePhysics` (`self.WeaponMesh`) false))))

(fn `StartAndEndPoint`
  (returns (Start :type "Vector Structure") (End :type "Vector Structure"))
  (locals (Range :type "Float (double-precision)"))
  (bind _followcamera (`/Game/ThirdPerson/Blueprints/BP_ThirdPersonCharacter.FollowCamera` (`self.PlayerRef`)))
  (return (+ (`SceneComponent.K2_GetComponentLocation` _followcamera) (`KismetMathLibrary.GetForwardVector` (`SceneComponent.K2_GetComponentRotation` _followcamera))) (+ (`SceneComponent.K2_GetComponentLocation` _followcamera) (* (`KismetMathLibrary.GetForwardVector` (`SceneComponent.K2_GetComponentRotation` _followcamera)) (`self.WeaponRange`)))))

(fn `UserConstructionScript`
  (bind (_weaponstruct_weaponname _weaponstruct_weaponenum _weaponstruct_weaponclass _weaponstruct_magsize _weaponstruct_currentammo _weaponstruct_damage _weaponstruct_weaponimage _weaponstruct_ismeleeweapon) (break `/Game/Blueprints/Weapons/WeaponStruc` (`self.weaponStruct`)))
  (setmembers `/Game/Blueprints/Weapons/WeaponStruc` :`StructRef` (`self.weaponStruct`) :`WeaponName` _weaponstruct_weaponname :`WeaponEnum` _weaponstruct_weaponenum :`WeaponClass` (`GameplayStatics.GetObjectClass` self) :`MagSize` _weaponstruct_magsize :`CurrentAmmo` _weaponstruct_currentammo :`Damage` _weaponstruct_damage :`WeaponImage` _weaponstruct_weaponimage :`isMeleeWeapon` _weaponstruct_ismeleeweapon))