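; Weapon inventory component for BP_ThirdPersonCharacter that handles pickup, drop, equip and holstering across primary, secondary, sidearm and melee slots.
; PickupWeapon routes by weapon type to holster checks, which choose an empty socket or drop a weapon and retry recursively.
; Attaching to a holster triggers auto-equip when nothing is equipped.
; EquipAndUnequip swaps mesh sockets, updating weapon state and equipped flags, while WeaponTypeAnim validates slot-switch requests.
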(event `self.ReceiveBeginPlay`
  (bind _asbp_third_person_character (cast `/Game/ThirdPerson/Blueprints/BP_ThirdPersonCharacter` (`GameplayStatics.GetPlayerCharacter` 0)))
  (set `self.PlayerRef` _asbp_third_person_character))

(event `EquipEvent`
  (bind _weaponinput (`self.WeaponInput`))
  (if (`|EnumInequality` (`self.WeaponInput`) "NewEnumerator0")
    (if (`self.HadWeaponEquipped`)
      _
      (elif (`|EnumInequality` _weaponinput "NewEnumerator5")
        (`self.EquipAndUnequip` (`self.InputBasedOnWeapons` _weaponinput) true)))))

(fn `AttachWeaponToPlayer`
  (params (Weapon :type "/Game/Blueprints/Weapons/MasterWeapon Object Reference") (Holster :type Name))
  (`Actor.K2_AttachToComponent` Weapon (`Character.Mesh` (`self.PlayerRef`)) Holster "SnapToTarget" "SnapToTarget" "SnapToTarget" true)
  (`/Game/Blueprints/Weapons/MasterWeapon.SetWeaponState` Weapon "NewEnumerator1")
  (bind _weaponslot (`self.GetSlotBasedOnWeapon` (`local.Weapon`)))
  (set `self.WeaponInput` _weaponslot)
  (`self.EquipEvent`))

(fn `DropWeapon`
  (params (WeaponToDrop :type "/Game/Blueprints/Weapons/MasterWeapon Object Reference"))
  (locals (WeaponSlot :type "/Game/Blueprints/Weapons/E_WeaponInput Enum" :default "NewEnumerator0"))
  (bind _weapontodrop (`local.WeaponToDrop`))
  (bind _weaponslot (`self.GetSlotBasedOnWeapon` WeaponToDrop))
  (set `local.WeaponSlot` _weaponslot)
  (`Actor.K2_DetachFromActor` _weapontodrop "KeepWorld" "KeepWorld" "KeepWorld")
  (`/Game/Blueprints/Weapons/MasterWeapon.SetWeaponState` _weapontodrop "NewEnumerator0")
  (set `self.WeaponInHand` null)
  (switch `/Game/Blueprints/Weapons/E_WeaponInput` (`local.WeaponSlot`)
    (:`NewEnumerator1`
      (set `self.PrimaryHolster` null)
      (set `self.RifleEquipped` false))
    (:`NewEnumerator2`
      (set `self.SecondaryHolster` null)
      (set `self.RifleEquipped` false))
    (:`NewEnumerator3`
      (set `self.SidearmHolster` null)
      (set `self.PistolEquipped` false))
    (:`NewEnumerator4`
      (set `self.MeleeHolster` null)
      (set `self.MeleeEquipped` false)))
  (return))

(fn `EquipAndUnequip`
  (params (Weapon :type "/Game/Blueprints/Weapons/MasterWeapon Object Reference") (WantToEquip :type Boolean))
  (locals (TheWeaponSlot :type "/Game/Blueprints/Weapons/E_WeaponInput Enum" :default "NewEnumerator0"))
  (bind _weaponslot (`self.GetSlotBasedOnWeapon` Weapon))
  (set `local.TheWeaponSlot` _weaponslot)
  (`Actor.K2_AttachToComponent` (`local.Weapon`) (`Character.Mesh` (`self.PlayerRef`)) (select `bool` (`local.WantToEquip`) :`false` (select `/Game/Blueprints/Weapons/E_WeaponInput` (`local.TheWeaponSlot`) :`NewEnumerator1` "holster_01" :`NewEnumerator2` "holster_02" :`NewEnumerator3` "holster_sidearm" :`NewEnumerator4` "holster_melee" :!type "Name") :`true` "holding") "SnapToTarget" "SnapToTarget" "SnapToTarget" true)
  (switch `/Game/Blueprints/Weapons/E_WeaponInput` (`local.TheWeaponSlot`)
    (:`NewEnumerator1`
      (set `self.RifleEquipped` true))
    (:`NewEnumerator2`
      (set `self.RifleEquipped` true))
    (:`NewEnumerator3`
      (set `self.PistolEquipped` true))
    (:`NewEnumerator4`
      (set `self.MeleeEquipped` true)))
  (if (`local.WantToEquip`)
    (bind _output_get (set `self.WeaponInHand` (`local.Weapon`)))
    (`/Game/Blueprints/Weapons/MasterWeapon.SetWeaponState` _output_get "NewEnumerator2")
    (return)
    (else
      (`/Game/Blueprints/Weapons/MasterWeapon.SetWeaponState` (`local.Weapon`) "NewEnumerator1")
      (set `self.RifleEquipped` false)
      (set `self.RifleEquipped` false)
      (set `self.PistolEquipped` false)
      (set `self.MeleeEquipped` false)
      (return))))

(fn `GetSlotBasedOnWeapon`
  (params (Weapon :type "/Game/Blueprints/Weapons/MasterWeapon Object Reference"))
  (returns (WeaponSlot :type "/Game/Blueprints/Weapons/E_WeaponInput Enum") (HolsterName :type Name))
  (if (and (`KismetSystemLibrary.IsValid` (`self.PrimaryHolster`)) (== (`local.Weapon`) (`self.PrimaryHolster`)))
    (return "NewEnumerator1" "holster_01")
    (elif (and (`KismetSystemLibrary.IsValid` (`self.SecondaryHolster`)) (== (`local.Weapon`) (`self.SecondaryHolster`)))
      (return "NewEnumerator2" "holster_02")
      (elif (and (`KismetSystemLibrary.IsValid` (`self.SidearmHolster`)) (== (`local.Weapon`) (`self.SidearmHolster`)))
        (return "NewEnumerator3" "holster_sidearm")
        (elif (and (`KismetSystemLibrary.IsValid` (`self.MeleeHolster`)) (== (`local.Weapon`) (`self.MeleeHolster`)))
          (return "NewEnumerator4" "holster_melee"))))))

(fn `HadWeaponEquipped`
  (returns (IsTrue :type Boolean))
  (return (or (`self.RifleEquipped`) (`self.PistolEquipped`) (`self.MeleeEquipped`))))

(fn `InputBasedOnWeapons`
  (params (WeaponInput :type "/Game/Blueprints/Weapons/E_WeaponInput Enum" :default "NewEnumerator0"))
  (returns (Weapon :type "/Game/Blueprints/Weapons/MasterWeapon Object Reference"))
  (bind _primaryholster (`self.PrimaryHolster`))
  (bind _secondaryholster (`self.SecondaryHolster`))
  (bind _sidearmholster (`self.SidearmHolster`))
  (bind _meleeholster (`self.MeleeHolster`))
  (bind _weaponinhand (`self.WeaponInHand`))
  (switch `/Game/Blueprints/Weapons/E_WeaponInput` WeaponInput
    (:`NewEnumerator1`
      (`/Engine/EditorBlueprintResources/StandardMacros.IsValid` _primaryholster
        (:`Is Valid`
          (return _primaryholster))))
    (:`NewEnumerator2`
      (`/Engine/EditorBlueprintResources/StandardMacros.IsValid` _secondaryholster
        (:`Is Valid`
          (return _secondaryholster))))
    (:`NewEnumerator3`
      (`/Engine/EditorBlueprintResources/StandardMacros.IsValid` _sidearmholster
        (:`Is Valid`
          (return _sidearmholster))))
    (:`NewEnumerator4`
      (`/Engine/EditorBlueprintResources/StandardMacros.IsValid` _meleeholster
        (:`Is Valid`
          (return _meleeholster))))
    (:`NewEnumerator5`
      (`/Engine/EditorBlueprintResources/StandardMacros.IsValid` _weaponinhand
        (:`Is Valid`
          (return _weaponinhand))))))

(fn `PickupWeapon`
  (params (weapon :type "/Game/Blueprints/Weapons/MasterWeapon Object Reference"))
  (locals (interactWeapon :type "/Game/Blueprints/Weapons/MasterWeapon Object Reference"))
  (bind _output_get (set `local.interactWeapon` weapon))
  (switch `/Game/Blueprints/Weapons/E_WeaponEnum` (`.WeaponEnum_5_0ADFDA6646BF9D63A3F0E09E4B430BED` (break `/Game/Blueprints/Weapons/WeaponStruc` (`/Game/Blueprints/Weapons/MasterWeapon.weaponStruct` _output_get)))
    (:`NewEnumerator0`
      (bind _theweapon (`self.CheckSidearmHolsterAvailability` (`local.interactWeapon`))
        (:`SidearmHolsterFull`
          (`self.PickupWeapon` (`local.interactWeapon`)))
        (:`SidearmHolsterEmpy`
          (bind _output_get_2 (set `self.SidearmHolster` _theweapon))
          (`self.AttachWeaponToPlayer` _output_get_2 (`self.EmptyHolster`)))))
    (:`NewEnumerator1`
      (bind _theweapon_2 (`self.CheckRifleHolsterAvailablity` (`local.interactWeapon`) :!label _label)
        (:`FullHolsters`
          (`self.PickupWeapon` (`local.interactWeapon`)))
        (:`SecondayHolsterEmpty`
          (bind _output_get_3 (set `self.SecondaryHolster` _theweapon_2))
          (`self.AttachWeaponToPlayer` _output_get_3 (`self.EmptyHolster`)))
        (:`PrimaryHolsterEmpty`
          (bind _output_get_4 (set `self.PrimaryHolster` _theweapon_2))
          (`self.AttachWeaponToPlayer` _output_get_4 (`self.EmptyHolster`)))))
    (:`NewEnumerator2`
      (goto _label))
    (:`NewEnumerator3`
      (goto _label))
    (:`NewEnumerator4`
      (bind _theweapon_3 (`self.CheckMeleeHolsterAvailability` (`local.interactWeapon`))
        (:`MeleeHolsterFull`
          (`self.PickupWeapon` (`local.interactWeapon`)))
        (:`MeleeHolsterEmpy`
          (bind _output_get_5 (set `self.MeleeHolster` _theweapon_3))
          (`self.AttachWeaponToPlayer` _output_get_5 (`self.EmptyHolster`)))))))

(fn `WeaponTypeAnim`
  (params (Weapon :type "/Game/Blueprints/Weapons/E_WeaponInput Enum" :default "NewEnumerator0"))
  (returns (CanAnimate :type Boolean))
  (bind _weaponinput (`self.WeaponInput`))
  (bind _weaponinhand (`self.WeaponInHand`))
  (switch `/Game/Blueprints/Weapons/E_WeaponInput` Weapon
    (:`NewEnumerator1`
      (`/Engine/EditorBlueprintResources/StandardMacros.IsValid` (`self.PrimaryHolster`)
        (:`Is Valid`
          _)
        (:`Is Not Valid`
          (set `self.WeaponInput` "NewEnumerator0" :!label _label)
          (return false))))
    (:`NewEnumerator2`
      (`/Engine/EditorBlueprintResources/StandardMacros.IsValid` (`self.SecondaryHolster`)
        (:`Is Valid`
          _)
        (:`Is Not Valid`
          (goto _label))))
    (:`NewEnumerator3`
      (`/Engine/EditorBlueprintResources/StandardMacros.IsValid` (`self.SidearmHolster`)
        (:`Is Valid`
          _)))
    (:`NewEnumerator4`
      (`/Engine/EditorBlueprintResources/StandardMacros.IsValid` (`self.MeleeHolster`)
        (:`Is Valid`
          _)
        (:`Is Not Valid`
          (goto _label))))
    (:`NewEnumerator5`
      (`/Engine/EditorBlueprintResources/StandardMacros.IsValid` (`self.WeaponInHand`)
        (:`Is Valid`
          (set `self.WeaponInput` "NewEnumerator0")
          (return true)))))
  (`/Engine/EditorBlueprintResources/StandardMacros.IsValid` _weaponinhand
    (:`Is Valid`
      (bind _weaponslot (`self.GetSlotBasedOnWeapon` _weaponinhand))
      (if (`|EnumEquality` _weaponslot _weaponinput)
        (set `self.WeaponInput` "NewEnumerator0")
        (return false)
        (else
          _)))
    (:`Is Not Valid`
      _))
  (set `self.WeaponInput` _weaponinput)
  (return true))